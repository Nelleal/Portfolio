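; BP_Button is a clickable world button that spawns a unit and sends it along a route from a spawn point to a finish, outlining itself on hover via custom depth.
; A valid click kills the previous unit, waits on the spawn effect, then spawns the configured class facing the finish.
; When the spawn montage blends out, the unit's AIC_Unit controller starts movement using the route type.
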(event OnBeginCursorOver(SM_Button)
  (params (TouchedComponent :type Primitive%20Component%20Object%20Reference))
  ;[1 1 1] Outline
  (Rendering|SetRenderCustomDepth (Variables|Default|GetSM_Button) true))

(event OnClicked(SM_Button)
  (params (TouchedComponent :type Primitive%20Component%20Object%20Reference) (ButtonPressed :type Key%20Structure :default "None"))
  ;[1 1 1] Click
  (bind _delay (CallFunction|CreateEffectonClick))
  (Utilities|FlowControl|Delay _delay)
  (if (CallFunction|GetButtonValid)
    (Utilities|IsValid (Variables|Default|GetUnitRef)
      (:Is%20Valid
        (Default|UnitDeath (Variables|Default|GetUnitRef)))
      (:Is%20Not%20Valid
        _))
    (CallFunction|SpawnUnit)))

(event OnEndCursorOver(SM_Button)
  (params (TouchedComponent :type Primitive%20Component%20Object%20Reference))
  ;[1 1 1] Outline
  (Rendering|SetRenderCustomDepth (Variables|Default|GetSM_Button) false))

(event Custom|SpawnUnit
  ;[1 1 1] SpawnUnit
  (bind (_delay _spawnlocation) (Default|CreateSpawnEffect (Variables|Init|GetSpawnRef)))
  (Utilities|FlowControl|Delay _delay)
  (bind _returnvalue (Game|SpawnActorfromClass (Variables|Init|GetUnit) (Math|Transform|MakeTransform _spawnlocation (Math|Conversions|RotationFromXVector (- (Transformation|GetWorldLocation (Variables|/Game/Project/Blueprints/BP_Finish.BP_Finish_C|GetDefaultSceneRoot (Variables|Init|GetFinishRef))) (Transformation|GetWorldLocation (Variables|/Game/Project/Blueprints/BP_Spawn.BP_Spawn_C|GetDefaultSceneRoot (Variables|Init|GetSpawnRef)))))) "Undefined" 0 0))
  (Variables|Default|SetUnitRef _returnvalue)
  (Animation|Montage|PlayMontage (Variables|/Script/Engine.Character|GetMesh (Variables|Default|GetUnitRef)) (.Value (Utilities|Map|Find (Variables|/Game/Project/Blueprints/BP_Unit.BP_Unit_C|GetAnimList (Variables|Default|GetUnitRef)) "NewEnumerator1"))
    (:OnBlendOut
      (CallFunction|StartMovement))))

(event Custom|StartMovement
  ;[1 1 1] StartMovement
  (bind _asaic_unit (Utilities|Casting|CastToAIC_Unit (AI|GetAIController (Variables|Default|GetUnitRef))))
  (Default|StartMovement _asaic_unit (Variables|Init|GetERouteType) (Variables|Default|GetUnitRef) (Variables|Init|GetSpawnRef) (Variables|Init|GetFinishRef)))

(event EventBeginPlay)

(fn ConstructionScript)

(fn CreateEffectonClick
  (return 0.0))

(fn GetButtonValid
  (if (Math|Boolean|ANDBoolean (Utilities|Enum|NotEqual(Enum) (Variables|Init|GetERouteType) "NewEnumerator0") (Math|Boolean|Equal(Boolean) (Utilities|IsValidClass (Variables|Init|GetUnit)) true) (Math|Boolean|Equal(Boolean) (Utilities|IsValid (Variables|Init|GetSpawnRef)) true) (Math|Boolean|Equal(Boolean) (Utilities|IsValid (Variables|Init|GetFinishRef)) true))
    (return true)
    (else
      (return false))))