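; BP_Unit is a unit actor that handles its own animation and sound feedback for spawning, idling, moving and dying.
; Animation events play montages looked up from the AnimList map by enum key, while BeginPlay plays the spawn sound.
; UnitDeath plays a sound, disables capsule and mesh collision, starts the death montage, tells AIC_Unit to end movement, and destroys the actor on montage blend-out.
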(event Custom|UnitDeath
  (Audio|PlaySound2D "/Game/Project/Assets/SoundEffects/A_Death.A_Death" 1.0 1.0 0.0 0 0)
  (Collision|SetCollisionResponsetoChannel (Variables|Collision|GetCapsuleComponent) "ECC_WorldStatic" "ECR_Ignore")
  (Collision|SetCollisionEnabled (Variables|Character|GetMesh) "NoCollision")
  (Animation|Montage|PlayMontage (Variables|Character|GetMesh) (.Value (Utilities|Map|Find (Variables|Default|GetAnimList) "NewEnumerator3"))
    (:then
      (bind _asaic_unit (Utilities|Casting|CastToAIC_Unit (AI|GetAIController self)))
      (Default|MovementEnd _asaic_unit))
    (:OnBlendOut
      (Actor|DestroyActor self))))

(event Custom|PlayAnimIdle
  (Animation|Montage|PlayMontage (Variables|Character|GetMesh) (.Value (Utilities|Map|Find (Variables|Default|GetAnimList) "NewEnumerator0"))))

(event Custom|PlayAnimSpawn
  (Animation|Montage|PlayMontage (Variables|Character|GetMesh) (.Value (Utilities|Map|Find (Variables|Default|GetAnimList) "NewEnumerator1"))))

(event Custom|PlayAnimMovement
  (Animation|Montage|PlayMontage (Variables|Character|GetMesh) (.Value (Utilities|Map|Find (Variables|Default|GetAnimList) "NewEnumerator2"))))

(event EventBeginPlay
  (Audio|PlaySound2D "/Game/Project/Assets/SoundEffects/A_Spawn.A_Spawn" 1.0 1.0 0.0 0 0))

(fn ConstructionScript)